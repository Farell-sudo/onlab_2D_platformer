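; BP_EnemyTurtle is a 2D flipbook enemy that periodically extends and retracts its spikes.
; A looping timer plays each transition flipbook, then flips the Spiked state after a delay matching its length.
; While spiked, capsule hits damage the player; otherwise, hits from above damage the turtle, with a brief DoOnce cooldown.
; It sets its max health on construction and destroys itself after the parent death logic.
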(event `self.ReceiveBeginPlay`
  (`KismetSystemLibrary.K2_SetTimerDelegate` (delegate `Animation Tick`) 5.0 true))

(event `Animation Tick`
  (if (`self.Spiked`)
    (`|ExecutionSequence`
      (:`then_0`
        (`PaperFlipbookComponent.SetFlipbook` (`self.Sprite`) "/Game/Assets/Flipbooks/Turtle/FB_Spikes_in.FB_Spikes_in"))
      (:`then_1`
        (`KismetSystemLibrary.Delay` (`PaperFlipbookComponent.GetFlipbookLength` (`self.Sprite`)))
        (`PaperFlipbookComponent.SetFlipbook` (`self.Sprite`) "/Game/Assets/Flipbooks/Turtle/FB_Idle_simple.FB_Idle_simple")
        (set `self.Spiked` (not (`self.Spiked`)))))
    (else
      (`|ExecutionSequence`
        (:`then_0`
          (`PaperFlipbookComponent.SetFlipbook` (`self.Sprite`) "/Game/Assets/Flipbooks/Turtle/FB_Spikes_out.FB_Spikes_out"))
        (:`then_1`
          (`KismetSystemLibrary.Delay` (`PaperFlipbookComponent.GetFlipbookLength` (`self.Sprite`)))
          (`PaperFlipbookComponent.SetFlipbook` (`self.Sprite`) "/Game/Assets/Flipbooks/Turtle/FB_Idle_spiked.FB_Idle_spiked")
          (set `self.Spiked` (not (`self.Spiked`))))))))

(event `self.ReceiveTick`
  (params (DeltaSeconds :type "Float (single-precision)")))

(event `self.CapsuleComponent.OnComponentHit`
  (params (HitComponent :type "PrimitiveComponent Object Reference") (OtherActor :type "Actor Object Reference") (OtherComp :type "PrimitiveComponent Object Reference") (NormalImpulse :type "Vector Structure") (Hit :type "HitResult Structure (by ref)"))
  (bind (_hitdirection_x _hitdirection_y _hitdirection_z) (`KismetMathLibrary.BreakVector` (`self.HitDirection`)))
  (set `self.HitRef` OtherActor)
  (`/Engine/EditorBlueprintResources/StandardMacros.DoOnce` false :!label _label
    (:`Completed`
      (set `self.HitDirection` (`KismetMathLibrary.Normal` (- Hit_Location (`self.K2_GetActorLocation`)) 0.0))
      (`|ExecutionSequence`
        (:`then_0`
          (if (and (`self.Spiked`) (== (`self.HitRef`) (`GameplayStatics.GetPlayerPawn` 0)))
            (`GameplayStatics.ApplyDamage` (`self.HitRef`) 20.0)
            (elif (>= _hitdirection_z 0.25)
              (`GameplayStatics.ApplyDamage` self 10.0 null (`GameplayStatics.GetPlayerPawn` 0)))))
        (:`then_1`
          (`KismetSystemLibrary.Delay` 0.1)
          (`self.REsetHitCheck`))))))

(event `ResetHitCheck`
  (goto _label :!via `Reset`))

(fn `ChangeState`)

(fn `EnemyDied`
  (`KismetSystemLibrary.PrintString` "Hello")
  (`parent.EnemyDied`)
  (`self.K2_DestroyActor`))

(fn `UserConstructionScript`
  (set `self.MaxHealth` 20.0)
  (`parent.UserConstructionScript`))