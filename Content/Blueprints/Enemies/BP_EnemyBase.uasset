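; BP_EnemyBase is a base enemy Blueprint that tracks health and detects death.
; The construction script sets ActualHealth to MaxHealth, and AnyDamage subtracts incoming damage, clamped between zero and that maximum.
; When health reaches zero, an IsDead guard ensures EnemyDied is called only once.
; EnemyDied is empty here, so this asset defines no death behavior of its own.
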(event `self.ReceiveAnyDamage`
  (params (Damage :type "Float (single-precision)") (DamageType :type "DamageType Object Reference") (InstigatedBy :type "Controller Object Reference") (DamageCauser :type "Actor Object Reference"))
  (set `self.ActualHealth` (`KismetMathLibrary.FClamp` (- (`self.ActualHealth`) Damage) 0.0 (`self.MaxHealth`)))
  (if (and (<= (`self.ActualHealth`) 0.0) (not (`self.isDead`)))
    (set `self.isDead` true)
    (`self.EnemyDied`)))

(fn `EnemyDied`)

(fn `UserConstructionScript`
  (set `self.ActualHealth` (`self.MaxHealth`)))