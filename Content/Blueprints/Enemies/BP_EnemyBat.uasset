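; Flying bat enemy for a 2D side-scroller that patrols along the X axis, starting in a random direction.
; Tick drives constant movement, while non-player hits with a horizontal normal reverse it and flip the sprite, debounced by a resettable DoOnce and short delay.
; Player hits on its upper part damage the bat by its full health; other player contact damages the player.
; It extends a parent enemy class and destroys itself on death.
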(event `self.ReceiveBeginPlay`
  (set `self.moveRight` (`KismetMathLibrary.RandomBool`))
  (`self.ToggleFacingDirection`))

(event `self.ReceiveTick`
  (params (DeltaSeconds :type "Float (single-precision)"))
  (`self.AddMovementInput` (1.0 0.0 0.0) (select `bool` (`self.moveRight`) :`false` -1.0 :`true` 1.0 :!type "Float (single-precision)")))

(event `self.CapsuleComponent.OnComponentHit`
  (params (HitComponent :type "PrimitiveComponent Object Reference") (OtherActor :type "Actor Object Reference") (OtherComp :type "PrimitiveComponent Object Reference") (NormalImpulse :type "Vector Structure") (Hit :type "HitResult Structure (by ref)"))
  (bind (_hitdirection_x _hitdirection_y _hitdirection_z) (`KismetMathLibrary.BreakVector` (`self.HitDirection`)))
  (bind _output_get (set `self.HitRef` OtherActor))
  (if (!= _output_get (`GameplayStatics.GetPlayerPawn` 0))
    (if (!= (`KismetMathLibrary.BreakVector3f` Hit_Normal) 0.0)
      (`/Engine/EditorBlueprintResources/StandardMacros.DoOnce` false :!label _label
        (:`Completed`
          (set `self.moveRight` (not (`self.moveRight`)))
          (`self.ToggleFacingDirection`)
          (`KismetSystemLibrary.Delay` 0.1)
          (`self.ResetDirectionChangeCheck`))))
    (else
      (set `self.HitDirection` (`KismetMathLibrary.Normal` (- Hit_Location (`self.K2_GetActorLocation`)) 0.0))
      (if (>= _hitdirection_z 0.25)
        (`GameplayStatics.ApplyDamage` self 10.0 null (`GameplayStatics.GetPlayerPawn` 0))
        (else
          (`GameplayStatics.ApplyDamage` (`self.HitRef`) 20.0))))))

(event `ResetDirectionChangeCheck`
  (goto _label :!via `Reset`))

(fn `EnemyDied`
  (`parent.EnemyDied`)
  (`self.K2_DestroyActor`))

(fn `ToggleFacingDirection`
  (bind (_returnvalue_x _returnvalue_y _returnvalue_z) (`KismetMathLibrary.BreakVector` (`SceneComponent.K2_GetComponentScale` (`self.Sprite`))))
  (`SceneComponent.SetWorldScale3D` (`self.Sprite`) (`KismetMathLibrary.MakeVector` (* (`KismetMathLibrary.Abs` _returnvalue_x) (select `bool` (`self.moveRight`) :`false` 1.0 :`true` -1.0)) _returnvalue_y _returnvalue_z)))

(fn `UserConstructionScript`
  (set `self.MaxHealth` 10.0)
  (`parent.UserConstructionScript`))